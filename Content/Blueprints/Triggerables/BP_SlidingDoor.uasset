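; BP_SlidingDoor is a triggerable double sliding door that opens and closes through Overlapped and UnOverlapped events.
; Overlapped plays the DoorOpenAmount timeline, which lerps the left and right door meshes' relative locations from the origin to their configured open positions.
; UnOverlapped reverses the same timeline from its current point to slide both panels shut.
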(event EventBeginPlay)

(event Collision|EventActorBeginOverlap
  (params (OtherActor :type Actor%20Object%20Reference)))

(event EventTick
  (params (DeltaSeconds :type Float%20%28single-precision%29)))

(event EventOverlapped
  (params (Other%20Actor :type Actor%20Object%20Reference))
  (bind _dooropenamount (Timeline|DoorOpenAmount Play)
    (:Update
      (Transformation|SetRelativeLocation (Variables|Default|GetSM_DoorLeft) (Math|Vector|Lerp(Vector) "0, 0, 0" (Variables|Default|GetL_DoorOpenPos) _dooropenamount) false false)
      (Transformation|SetRelativeLocation (Variables|Default|GetSM_DoorRight) (Math|Vector|Lerp(Vector) "0, 0, 0" (Variables|Default|GetR_DoorOpenPos) _dooropenamount) false false))))

(event EventUnOverlapped
  (params (Other%20Actor :type Actor%20Object%20Reference))
  (bind _dooropenamount (Timeline|DoorOpenAmount Reverse)
    (:Update
      (Transformation|SetRelativeLocation (Variables|Default|GetSM_DoorLeft) (Math|Vector|Lerp(Vector) "0, 0, 0" (Variables|Default|GetL_DoorOpenPos) _dooropenamount) false false)
      (Transformation|SetRelativeLocation (Variables|Default|GetSM_DoorRight) (Math|Vector|Lerp(Vector) "0, 0, 0" (Variables|Default|GetR_DoorOpenPos) _dooropenamount) false false))))

(fn ConstructionScript
  (|CallParentFunction))